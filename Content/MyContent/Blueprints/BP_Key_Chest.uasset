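; BP_Key_Chest is a key pickup that stays hidden and non-collidable until no BP_Target actors remain in the level.
; Tick polls for targets every frame to drive mesh visibility and actor collision, with a DoOnce firing a spawn effect and sound when the key appears.
; Player overlap then sets HasKey on the cached BP_FirstPersonCharacter, plays a ping and destroys the key.
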(event OnComponentBeginOverlap(Collision)
  (params (OverlappedComponent :type Primitive%20Component%20Object%20Reference) (OtherActor :type Actor%20Object%20Reference) (OtherComp :type Primitive%20Component%20Object%20Reference) (OtherBodyIndex :type Integer) (bFromSweep :type Boolean) (SweepResult :type Hit%20Result%20Structure%20%28by%20ref%29))
  ;[0.08463 0.1194 0.15 0.5] Collecting the Key
  (if (and (== OtherActor (Variables|Default|GetBP_FirstPersonCharacter)) (Variables|Default|GetAllTargetsDestroyed))
    (Variables|/Game/StarterContent/FirstPerson/Blueprints/BP_FirstPersonCharacter.BP_FirstPersonCharacter_C|SetHasKey (Variables|Default|GetBP_FirstPersonCharacter) true)
    (Audio|PlaySoundatLocation "/Engine/EngineSounds/1kSineTonePing.1kSineTonePing" (Transformation|GetActorLocation) "0, 0, 0" 1.0 1.0 0.0 0 0 0 0)
    (Actor|DestroyActor)))

(event EventBeginPlay
  ;[0.15 0.1333 0.07891 0.5] Setup
  (bind _asbp_first_person_character (Utilities|Casting|CastToBP_FirstPersonCharacter (Game|GetPlayerCharacter 0)))
  (Variables|Default|SetBP_FirstPersonCharacter _asbp_first_person_character))

(event Collision|EventActorBeginOverlap
  (params (OtherActor :type Actor%20Object%20Reference)))

(event EventTick
  (params (DeltaSeconds :type Float%20%28single-precision%29))
  (bind _sm_key (Variables|Default|GetSM_Key))
  (bind _returnvalue (Transformation|GetWorldLocation _sm_key))
  ;[0.0763 0.15 0.1213 0.5] Key Visibility
  (bind _outactors (Actor|GetAllActorsOfClass "/Game/MyContent/Blueprints/BP_Target.BP_Target_C"))
  (bind _returnvalue_2 (Utilities|Array|Add _outactors 0))
  (bind _output_get (Variables|Default|SetAllTargetsDestroyed (<= _returnvalue_2 0)))
  (Rendering|SetVisibility (Variables|Default|GetSM_Key) _output_get true)
  (Collision|SetActorEnableCollision _output_get)
  ;[0.1238 0.06897 0.151 0.5] Show Key Effects
  (if (Variables|Default|GetAllTargetsDestroyed)
    (Utilities|FlowControl|DoOnce false
      (:Completed
        (Niagara|SpawnSystematLocation 0 _returnvalue "0, 0, 0" "1.000000,1.000000,1.000000" true true "AutoRelease")
        (Audio|SpawnSoundatLocation "/Engine/VREditor/Sounds/UI/Leave_Simulate.Leave_Simulate" _returnvalue "0, 0, 0" 1.0 1.0 0.0 0 0)))))

(fn ConstructionScript)